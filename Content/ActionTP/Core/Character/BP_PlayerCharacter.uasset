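; Player character Blueprint for ActionTP that sets up the player's HUD and exposes health for debugging.
; On BeginPlay it creates the crosshair and player health widgets and adds both to the viewport.
; It prints the AttributeComponent's current health to screen every Tick, and prints the new value in red whenever OnHealthChanged fires.
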(event `self.ReceiveBeginPlay`
  (bind _returnvalue (`|CreateWidget` "/Game/ActionTP/Core/UI/WBP_Crosshair.WBP_Crosshair_C"))
  (`UserWidget.AddToViewport` _returnvalue 0)
  (bind _returnvalue_2 (`|CreateWidget` "/Game/ActionTP/Core/UI/WBP_PlayerHealth.WBP_PlayerHealth_C"))
  (`UserWidget.AddToViewport` _returnvalue_2 0))

(event `self.ReceiveTick`
  (params (DeltaSeconds :type "Float (single-precision)"))
  (`KismetSystemLibrary.PrintString` (`KismetStringLibrary.Conv_DoubleToString` (`SAttributeComponent.Health` (`self.AttributeComponent`))) true false (struct :`G` 0.66 :`B` 1.0 :`A` 1.0) 0.0))

(event `self.AttributeComponent.OnHealthChanged`
  (params (InstigatorActor :type "Actor Object Reference") (OwningComponent :type "SAttributeComponent Object Reference") (NewHealth :type "Float (single-precision)") (Delta :type "Float (single-precision)"))
  (`KismetSystemLibrary.PrintString` (`KismetStringLibrary.Conv_DoubleToString` NewHealth) true true (struct :`R` 1.0 :`G` 0.116117 :`B` 0.235884 :`A` 1.0)))

(fn `UserConstructionScript`)